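; Enemy spawner actor that spawns kamikaze enemies at its own transform and reports their destruction to BP_FirstPersonGameMode.
; AddEnemyToQueue queues a class and spawns immediately if no kamikaze overlaps the Sphere, while a looping timer also retries.
; SpawnEnemy consumes one queue entry per attempt, even if collision blocks it, and always uses BP_Enemy_Kamikaze regardless of queued class.
; The spawn particle effect is defined but never runs.
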(event Custom|OnEnemyDefeated
  (params (DestroyedActor :type Actor%20Object%20Reference))
  (bind _asbp_first_person_game_mode (Utilities|Casting|CastToBP_FirstPersonGameMode (Game|GetGameMode)))
  (Default|OnEnemyDefeated _asbp_first_person_game_mode))

(event Custom|TryToSpawn
  (CallFunction|SpawnEnemy))

(event EventBeginPlay
  (Utilities|Time|SetTimerbyEvent (delegate Custom|TryToSpawn) 2.0 true))

(event Collision|EventActorBeginOverlap
  (params (OtherActor :type Actor%20Object%20Reference)))

(fn ConstructionScript)

(fn SpawnParticleEffect
  (Niagara|SpawnSystematLocation "/Game/Art/VFX/NiagaraSystems/NS_Spawn.NS_Spawn" (+ (Transformation|GetSocketLocation (Variables|Default|GetCube) "None") "0.000000,0.000000,10.000000")))

(fn SpawnEnemy
  (if (Utilities|Array|IsValidIndex (Variables|Default|GetEnemyQueue))
    (bind _returnvalue (Game|SpawnActorfromClass "/Game/Blueprints/Enemy/BP_Enemy_Kamikaze.BP_Enemy_Kamikaze_C" (Transformation|GetActorTransform) "AdjustIfPossibleButDontSpawnIfColliding" "MultiplyWithRoot" 0 0))
    (Game|BindEventtoOnDestroyed _returnvalue (EventDispatchers|CreateEvent :!event Custom|OnEnemyDefeated))
    (Utilities|Array|RemoveIndex (Variables|Default|GetEnemyQueue))
    (return true)
    (else
      (return false))))

(fn AddEnemytoQueue
  (params (EnemyClass :type BP%20Enemy%20Kamikaze%20Class%20Reference%20%28by%20ref%29))
  (Utilities|Array|Add (Variables|Default|GetEnemyQueue) EnemyClass)
  (if (not (Utilities|Array|IsValidIndex (Collision|GetOverlappingActors (Variables|Default|GetSphere) "/Game/Blueprints/Enemy/BP_Enemy_Kamikaze.BP_Enemy_Kamikaze_C" :!class /Script/Engine.PrimitiveComponent)))
    (CallFunction|SpawnEnemy)))