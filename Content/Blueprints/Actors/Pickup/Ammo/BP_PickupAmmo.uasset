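; Ammo pickup actor that refills a weapon of the first-person character when it overlaps the box, then respawns.
; It grants ammo to only the first owned weapon in plasma rifle, shotgun, rocket launcher order, locating it via GetActorOfClass.
; After playing a sound, it hides the cone and blocks pickup for a fixed delay before restoring both.
; A randomized-delay respawn chain is left unconnected.
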(event OnComponentBeginOverlap(Box)
  (params (OverlappedComponent :type Primitive%20Component%20Object%20Reference) (OtherActor :type Actor%20Object%20Reference) (OtherComp :type Primitive%20Component%20Object%20Reference) (OtherBodyIndex :type Integer) (bFromSweep :type Boolean) (SweepResult :type Hit%20Result%20Structure%20%28by%20ref%29))
  (bind _cone (Variables|Default|GetCone))
  (if (not (Variables|Default|GetIsOnCooldown))
    (bind _asbp_first_person_character (Utilities|Casting|CastToBP_FirstPersonCharacter OtherActor))
    (if (Variables|/Game/FirstPerson/Blueprints/BP_FirstPersonCharacter.BP_FirstPersonCharacter_C|GethasPlasmaRifle? _asbp_first_person_character)
      (bind _returnvalue (Actor|GetActorOfClass "/Game/FirstPerson/Blueprints/Weapons/Shotgun/BP_Weapon_PlasmaRifle.BP_Weapon_PlasmaRifle_C"))
      (Variables|/Game/FirstPerson/Blueprints/Weapons/Shotgun/BP_Weapon_PlasmaRifle.BP_Weapon_PlasmaRifle_C|SetPlasmaAmmo _returnvalue (+ (Variables|/Game/FirstPerson/Blueprints/Weapons/Shotgun/BP_Weapon_PlasmaRifle.BP_Weapon_PlasmaRifle_C|GetPlasmaAmmo _returnvalue) 50))
      (Audio|PlaySound2D "/Game/Project/Sounds/SFX_AMMO_PICKUP.SFX_AMMO_PICKUP" 1.0 1.0 0.0 0 0)
      (Rendering|SetVisibility _cone false false :!label _label)
      (Variables|Default|SetIsOnCooldown true)
      (Utilities|FlowControl|Delay 15.0)
      (Variables|Default|SetIsOnCooldown false)
      (Rendering|SetVisibility _cone true false)
      (elif (Variables|/Game/FirstPerson/Blueprints/BP_FirstPersonCharacter.BP_FirstPersonCharacter_C|GethasShotgun? _asbp_first_person_character)
        (bind _returnvalue_2 (Actor|GetActorOfClass "/Game/FirstPerson/Blueprints/Weapons/Shotgun/BP_Weapon_Shotgun.BP_Weapon_Shotgun_C"))
        (Variables|/Game/FirstPerson/Blueprints/Weapons/Shotgun/BP_Weapon_Shotgun.BP_Weapon_Shotgun_C|SetShotgunAmmo _returnvalue_2 (+ (Variables|/Game/FirstPerson/Blueprints/Weapons/Shotgun/BP_Weapon_Shotgun.BP_Weapon_Shotgun_C|GetShotgunAmmo _returnvalue_2) 10))
        (Audio|PlaySound2D "/Game/Project/Sounds/SFX_AMMO_PICKUP.SFX_AMMO_PICKUP" 1.0 1.0 0.0 0 0)
        (goto _label)
        (elif (Variables|/Game/FirstPerson/Blueprints/BP_FirstPersonCharacter.BP_FirstPersonCharacter_C|GethasRocketLauncher? _asbp_first_person_character)
          (bind _returnvalue_3 (Actor|GetActorOfClass "/Game/FirstPerson/Blueprints/Weapons/Shotgun/BP_Weapon_RocketLauncher.BP_Weapon_RocketLauncher_C"))
          (Variables|/Game/FirstPerson/Blueprints/Weapons/Shotgun/BP_Weapon_RocketLauncher.BP_Weapon_RocketLauncher_C|SetRocketAmmo _returnvalue_3 (+ (Variables|/Game/FirstPerson/Blueprints/Weapons/Shotgun/BP_Weapon_RocketLauncher.BP_Weapon_RocketLauncher_C|GetRocketAmmo _returnvalue_3) 4))
          (Audio|PlaySound2D "/Game/Project/Sounds/SFX_AMMO_PICKUP.SFX_AMMO_PICKUP" 1.0 1.0 0.0 0 0)
          (goto _label))))))

(event EventBeginPlay
  (|CallParentFunction) ; This node is disabled and will not be called.\nDrag off pins to build functionality.
)

(event Collision|EventActorBeginOverlap
  (params (OtherActor :type Actor%20Object%20Reference))
  (|CallParentFunction OtherActor) ; This node is disabled and will not be called.\nDrag off pins to build functionality.
)

(event EventTick
  (params (DeltaSeconds :type Float%20%28single-precision%29))
  (|CallParentFunction DeltaSeconds) ; This node is disabled and will not be called.\nDrag off pins to build functionality.
)

(fn ConstructionScript
  (|CallParentFunction))