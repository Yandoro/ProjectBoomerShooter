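; Flying drone enemy that fires BP_FlyingEnemyProjectile at the first-person player about once a second, via a Delay on Tick.
; Shots lead the target using player velocity scaled by distance.
; Each tick also moves the Cable end to the player and runs a line trace whose result is unused.
; HitEnemy reduces Health but only prints on death; AnyDamage only prints and RotateDrone is empty.
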(event Custom|LINETRACE
  (bind _playerref (Variables|Default|GetPlayerRef))
  (Collision|LineTraceByChannel (Transformation|GetWorldLocation (Variables|Default|GetProjectileSpawn)) (+ (Transformation|GetWorldLocation (Variables|/Script/Engine.Actor|GetRootComponent _playerref)) (* (Transformation|GetVelocity _playerref) (/ (Transformation|GetDistanceTo _playerref) 4.5e+03))) "TraceTypeQuery1" false 0 "None")
  (Variables|/Script/CableComponent.CableComponent|SetEndLocation (Variables|Default|GetCable) (Math|Transform|InverseTransformLocation (Transformation|GetActorTransform) (Transformation|GetWorldLocation (Variables|/Script/Engine.Actor|GetRootComponent (Variables|Default|GetPlayerRef))))))

(event EventBeginPlay
  (bind _asbp_first_person_character (Utilities|Casting|CastToBP_FirstPersonCharacter (Game|GetPlayerCharacter 0)))
  (Variables|Default|SetPlayerRef _asbp_first_person_character))

(event Collision|EventActorBeginOverlap
  (params (OtherActor :type Actor%20Object%20Reference)))

(event Game|Damage|EventAnyDamage
  (params (Damage :type Float%20%28single-precision%29) (DamageType :type Damage%20Type%20Object%20Reference) (InstigatedBy :type Controller%20Object%20Reference) (DamageCauser :type Actor%20Object%20Reference))
  (Development|PrintString "ERHALTEN"))

(event EventTick
  (params (DeltaSeconds :type Float%20%28single-precision%29))
  (bind _playerref (Variables|Default|GetPlayerRef))
  (bind _projectilespawn (Variables|Default|GetProjectileSpawn))
  (bind _returnvalue (Transformation|GetWorldLocation _projectilespawn))
  (bind _rootcomponent (Variables|/Script/Engine.Actor|GetRootComponent _playerref))
  (bind _returnvalue_2 (Transformation|GetWorldLocation _rootcomponent))
  (CallFunction|LINETRACE)
  (CallFunction|RotateDrone)
  (Utilities|FlowControl|Delay 1.0)
  (Transformation|SetRelativeRotation (Variables|Default|GetProjectileSpawn) (Math|Rotator|FindLookatRotation _returnvalue _returnvalue_2) false false)
  (Game|SpawnActorfromClass "/Game/FirstPerson/Blueprints/BP_FlyingEnemyProjectile.BP_FlyingEnemyProjectile_C" (Math|Transform|MakeTransform _returnvalue (Math|Rotator|FindLookatRotation _returnvalue (+ _returnvalue_2 (* (Transformation|GetVelocity _playerref) (/ (Transformation|GetDistanceTo _playerref) 4.5e+03))))) "Undefined" "MultiplyWithRoot" 0 0))

(event EventHitEnemy
  (params (Damage :type Float%20%28double-precision%29))
  (bind _output_get (Variables|Default|SetHealth (- (Variables|Default|GetHealth) Damage)))
  (if (<= _output_get 0.0)
    (Development|PrintString "EnemeyKilled")))

(fn ConstructionScript)

(fn RotateDrone)