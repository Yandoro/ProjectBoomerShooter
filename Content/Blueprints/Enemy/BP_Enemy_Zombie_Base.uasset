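; Base zombie enemy character that chases the player through blackboard flags, dissolves on spawn and ragdolls on death.
; BeginPlay sets the chaser flag, PawnSensing updates player sight, and a sphere overlap lowers walk speed near the player.
; Timelines drive dissolve materials on both mesh slots, and Damage decrements health before ragdoll, dissolve and destruction.
; JumptoDestination launches it along a computed arc; an AIMoveTo loop is left unconnected.
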(event OnSeePawn(PawnSensing)
  (params (Pawn :type Pawn%20Object%20Reference))
  (bind _returnvalue (Utilities|Name|MakeLiteralName "BT_CanSeePlayer"))
  (bind _self self)
  (bind _returnvalue_2 (AI|GetAIController _self))
  (bind _returnvalue_3 (AI|GetBlackboard _returnvalue_2))
  ;[1 1 1] PawnSensing
  (Utilities|Casting|CastToBP_FirstPersonCharacter Pawn
    (:then
      (AI|Components|Blackboard|SetValueasBool _returnvalue_3 _returnvalue true))
    (:CastFailed
      (AI|Components|Blackboard|SetValueasBool _returnvalue_3 _returnvalue false))))

(event OnComponentBeginOverlap(Sphere)
  (params (OverlappedComponent :type Primitive%20Component%20Object%20Reference) (OtherActor :type Actor%20Object%20Reference) (OtherComp :type Primitive%20Component%20Object%20Reference) (OtherBodyIndex :type Integer) (bFromSweep :type Boolean) (SweepResult :type Hit%20Result%20Structure%20%28by%20ref%29))
  (Utilities|Casting|CastToBP_FirstPersonCharacter OtherActor)
  (Variables|/Script/Engine.CharacterMovementComponent|SetMaxWalkSpeed (Variables|Character|GetCharacterMovement) 7.5e+02))

(event OnComponentEndOverlap(Sphere)
  (params (OverlappedComponent :type Primitive%20Component%20Object%20Reference) (OtherActor :type Actor%20Object%20Reference) (OtherComp :type Primitive%20Component%20Object%20Reference) (OtherBodyIndex :type Integer))
  (Utilities|Casting|CastToBP_FirstPersonCharacter OtherActor)
  (Variables|/Script/Engine.CharacterMovementComponent|SetMaxWalkSpeed (Variables|Character|GetCharacterMovement) 1.5e+03))

(event Custom|Damage
  (Variables|Default|SetEnemyHealth (- (Variables|Default|GetEnemyHealth) 1))
  (if (not (> (Variables|Default|GetEnemyHealth) 1))
    (Physics|SetSimulatePhysics (Variables|Character|GetMesh) true)
    (CallFunction|2)
    (Collision|SetCollisionEnabled (Variables|Collision|GetCapsuleComponent) "NoCollision")
    (bind _returnvalue (Rendering|Material|CreateDynamicMaterialInstance (Variables|Character|GetMesh) 0 "/Game/Blueprints/Enemy/MI_DissolveMaterial_Inst.MI_DissolveMaterial_Inst" "None" :!class /Script/Engine.PrimitiveComponent))
    (bind _newtrack_0 (Timeline|Timeline_0 Play)
      (:Update
        (Rendering|Material|SetScalarParameterValue _returnvalue "Progress" _newtrack_0 :!class /Script/Engine.MaterialInstanceDynamic)
        (Utilities|FlowControl|Delay 1.5)
        (Actor|DestroyActor)))))

(event Custom|2
  (bind _returnvalue (Rendering|Material|CreateDynamicMaterialInstance (Variables|Character|GetMesh) 1 "/Game/Blueprints/Enemy/MI_DissolveMaterial_Inst.MI_DissolveMaterial_Inst" "None" :!class /Script/Engine.PrimitiveComponent))
  (bind _newtrack_0 (Timeline|Timeline Play)
    (:Update
      (Rendering|Material|SetScalarParameterValue _returnvalue "Progress" _newtrack_0 :!class /Script/Engine.MaterialInstanceDynamic))))

(event Custom|SpawnEffect
  (CallFunction|Second)
  (bind _returnvalue (Rendering|Material|CreateDynamicMaterialInstance (Variables|Character|GetMesh) 0 "/Game/Blueprints/Enemy/M_DissolveMaterial.M_DissolveMaterial" "None" :!class /Script/Engine.PrimitiveComponent))
  (bind _newtrack_0 (Timeline|Timeline_1 Play)
    (:Update
      (Rendering|Material|SetScalarParameterValue _returnvalue "Progress" _newtrack_0 :!class /Script/Engine.MaterialInstanceDynamic)
      (Utilities|FlowControl|Delay 1.5)
      (Rendering|Material|SetMaterial (Variables|Character|GetMesh) 0 "/Game/Project/DefaultStuff/Characters/Mannequins/Materials/Instances/Quinn/MI_Quinn_01.MI_Quinn_01"))))

(event Custom|Second
  (bind _returnvalue (Rendering|Material|CreateDynamicMaterialInstance (Variables|Character|GetMesh) 1 "/Game/Blueprints/Enemy/M_DissolveMaterial.M_DissolveMaterial" "None" :!class /Script/Engine.PrimitiveComponent))
  (bind _newtrack_0 (Timeline|Timeline_2 Play)
    (:Update
      (Rendering|Material|SetScalarParameterValue _returnvalue "Progress" _newtrack_0 :!class /Script/Engine.MaterialInstanceDynamic)
      (Utilities|FlowControl|Delay 1.5)
      (Rendering|Material|SetMaterial (Variables|Character|GetMesh) 1 "/Game/Project/DefaultStuff/Characters/Mannequins/Materials/Instances/Quinn/MI_Quinn_02.MI_Quinn_02"))))

(event EventJumptoDestination
  (params (Destination :type Vector :default "0, 0, 0"))
  (bind (_x _y _z) (Math|Vector|BreakVector Destination))
  (bind _outlaunchvelocity (Game|SuggestProjectileVelocityCustomArc (Transformation|GetActorLocation) (Math|Vector|MakeVector _x _y (+ _z 3e+02)) 0.0 0.5))
  (Character|LaunchCharacter _outlaunchvelocity true true))

(event EventBeginPlay
  (AI|Components|Blackboard|SetValueasBool (AI|GetBlackboard (AI|GetAIController self)) (Utilities|Name|MakeLiteralName "BT_Chaser") true)
  (CallFunction|SpawnEffect)
  (Utilities|FlowControl|Delay 0.2))

(fn ConstructionScript)