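; Flying drone enemy that pursues the first-person player and shoots projectiles at them.
; ProjectileMovement homes on the player's capsule, dropping to near-zero max speed while the player is inside Sphere1.
; Tick smoothly turns the drone toward the player and, throttled by a one-second Delay, fires BP_FlyingEnemyProjectile with distance-based velocity lead.
; AnyDamage reduces Health and destroys the drone with an explosion when low; HitEnemy only prints on death.
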(event OnComponentBeginOverlap(Sphere1)
  (params (OverlappedComponent :type Primitive%20Component%20Object%20Reference) (OtherActor :type Actor%20Object%20Reference) (OtherComp :type Primitive%20Component%20Object%20Reference) (OtherBodyIndex :type Integer) (bFromSweep :type Boolean) (SweepResult :type Hit%20Result%20Structure%20%28by%20ref%29))
  (bind _projectilemovement (Variables|Default|GetProjectileMovement))
  (if (Actor|ActorHasTag OtherActor "Player")
    (Variables|/Script/Engine.ProjectileMovementComponent|SetInitialSpeed _projectilemovement 1.0)
    (Variables|/Script/Engine.ProjectileMovementComponent|SetMaxSpeed _projectilemovement 1.0)))

(event OnComponentEndOverlap(Sphere1)
  (params (OverlappedComponent :type Primitive%20Component%20Object%20Reference) (OtherActor :type Actor%20Object%20Reference) (OtherComp :type Primitive%20Component%20Object%20Reference) (OtherBodyIndex :type Integer))
  (bind _projectilemovement (Variables|Default|GetProjectileMovement))
  (if (Actor|ActorHasTag OtherActor "Player")
    (Variables|/Script/Engine.ProjectileMovementComponent|SetInitialSpeed _projectilemovement 4e+02)
    (Variables|/Script/Engine.ProjectileMovementComponent|SetMaxSpeed _projectilemovement 4e+02)))

(event Collision|EventActorBeginOverlap
  (params (OtherActor :type Actor%20Object%20Reference)))

(event Game|Damage|EventAnyDamage
  (params (Damage :type Float%20%28single-precision%29) (DamageType :type Damage%20Type%20Object%20Reference) (InstigatedBy :type Controller%20Object%20Reference) (DamageCauser :type Actor%20Object%20Reference))
  (Development|PrintString "Hello")
  (Variables|Default|SetHealth (- (Variables|Default|GetHealth) Damage))
  (if (not (> (Variables|Default|GetHealth) 1.0))
    (Components|DestroyComponent (Variables|Default|GetProjectileMovement))
    (Effects|SpawnEmitteratLocation "/Game/Project/DefaultStuff/StarterContent/Particles/P_Explosion.P_Explosion" (Transformation|GetSocketLocation (Variables|Default|GetSci-fi_Dron-Scorpion-42) "None") "0, 0, 0" "4.000000,4.000000,4.000000")
    (Actor|DestroyActor)))

(event EventTick
  (params (DeltaSeconds :type Float%20%28single-precision%29))
  (bind _projectilespawn (Variables|Default|GetProjectileSpawn))
  (bind _playerref (Variables|Default|GetPlayerRef))
  (bind _returnvalue (Transformation|GetWorldLocation _projectilespawn))
  (bind _rootcomponent (Variables|/Script/Engine.Actor|GetRootComponent _playerref))
  (bind _returnvalue_2 (Transformation|GetWorldLocation _rootcomponent))
  (CallFunction|RotateDrone)
  (Utilities|FlowControl|Delay 1.0)
  (Transformation|SetRelativeRotation (Variables|Default|GetProjectileSpawn) (Math|Rotator|FindLookatRotation _returnvalue _returnvalue_2) false false)
  (Game|SpawnActorfromClass "/Game/FirstPerson/Blueprints/BP_FlyingEnemyProjectile.BP_FlyingEnemyProjectile_C" (Math|Transform|MakeTransform _returnvalue (Math|Rotator|FindLookatRotation _returnvalue (+ _returnvalue_2 (* (Transformation|GetVelocity _playerref) (/ (Transformation|GetDistanceTo _playerref) 4.5e+03))))) "Undefined" "MultiplyWithRoot" 0 0))

(event EventHitEnemy
  (params (Damage :type Float%20%28double-precision%29))
  (bind _output_get (Variables|Default|SetHealth (- (Variables|Default|GetHealth) Damage)))
  (if (<= _output_get 0.0)
    (Development|PrintString "EnemeyKilled")))

(event EventBeginPlay
  (bind _asbp_first_person_character (Utilities|Casting|CastToBP_FirstPersonCharacter (Game|Player|GetPlayerPawn 0)))
  (Variables|Default|SetPlayerRef _asbp_first_person_character)
  (Variables|/Script/Engine.ProjectileMovementComponent|SetHomingTargetComponent (Variables|Default|GetProjectileMovement) (Variables|/Script/Engine.Character|GetCapsuleComponent _asbp_first_person_character)))

(fn ConstructionScript)

(fn RotateDrone
  (bind _returnvalue (Game|Player|GetPlayerPawn 0))
  (bind _returnvalue_2 (Utilities|Time|GetWorldDeltaSeconds))
  (bind _returnvalue_3 (Transformation|GetActorLocation))
  (bind _returnvalue_4 (Transformation|GetActorRotation))
  (bind _returnvalue_5 (Transformation|GetActorLocation _returnvalue))
  (bind _returnvalue_6 (Math|Rotator|FindLookatRotation _returnvalue_3 _returnvalue_5))
  (bind _returnvalue_7 (Math|Interpolation|RInterpTo _returnvalue_4 _returnvalue_6 _returnvalue_2 3.0))
  (Transformation|SetActorRotation self (Math|Rotator|MakeRotator (.roll _returnvalue_7) (.pitch _returnvalue_7) (.yaw _returnvalue_7))))