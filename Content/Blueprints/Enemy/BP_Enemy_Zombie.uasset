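; Zombie enemy that dissolves in on spawn, repeatedly moves toward the player character via AI MoveTo, and dissolves away on death.
; Timelines drive the Progress parameter of dynamic dissolve materials on both mesh slots, with regular Quinn materials restored after the spawn effect.
; Damage decrements health and triggers death at one or below; the spawn chain also calls death after delays.
; Death enables ragdoll physics, disables capsule collision and destroys the actor.
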(event Custom|Damage
  (Variables|Default|SetEnemyHealth (- (Variables|Default|GetEnemyHealth) 1))
  (if (not (> (Variables|Default|GetEnemyHealth) 1))
    (Physics|SetSimulatePhysics (Variables|Character|GetMesh) true)
    (CallFunction|2)
    (Collision|SetCollisionEnabled (Variables|Collision|GetCapsuleComponent) "NoCollision")
    (bind _returnvalue (Rendering|Material|CreateDynamicMaterialInstance (Variables|Character|GetMesh) 0 "/Game/Blueprints/Enemy/MI_DissolveMaterial_Inst.MI_DissolveMaterial_Inst" "None" :!class /Script/Engine.PrimitiveComponent))
    (bind _newtrack_0 (Timeline|Timeline_0 Play)
      (:Update
        (Rendering|Material|SetScalarParameterValue _returnvalue "Progress" _newtrack_0 :!class /Script/Engine.MaterialInstanceDynamic)
        (Utilities|FlowControl|Delay 1.5)
        (Actor|DestroyActor)))))

(event Custom|2
  (bind _returnvalue (Rendering|Material|CreateDynamicMaterialInstance (Variables|Character|GetMesh) 1 "/Game/Blueprints/Enemy/MI_DissolveMaterial_Inst.MI_DissolveMaterial_Inst" "None" :!class /Script/Engine.PrimitiveComponent))
  (bind _newtrack_0 (Timeline|Timeline Play)
    (:Update
      (Rendering|Material|SetScalarParameterValue _returnvalue "Progress" _newtrack_0 :!class /Script/Engine.MaterialInstanceDynamic))))

(event Custom|SpawnEffect
  (CallFunction|Second)
  (bind _returnvalue (Rendering|Material|CreateDynamicMaterialInstance (Variables|Character|GetMesh) 0 "/Game/Blueprints/Enemy/M_DissolveMaterial.M_DissolveMaterial" "None" :!class /Script/Engine.PrimitiveComponent))
  (bind _newtrack_0 (Timeline|Timeline_1 Play)
    (:Update
      (Rendering|Material|SetScalarParameterValue _returnvalue "Progress" _newtrack_0 :!class /Script/Engine.MaterialInstanceDynamic)
      (Utilities|FlowControl|Delay 1.5)
      (Rendering|Material|SetMaterial (Variables|Character|GetMesh) 0 "/Game/Project/DefaultStuff/Characters/Mannequins/Materials/Instances/Quinn/MI_Quinn_01.MI_Quinn_01")
      (Utilities|FlowControl|Delay 3.0)
      (CallFunction|Ded))))

(event Custom|Second
  (bind _returnvalue (Rendering|Material|CreateDynamicMaterialInstance (Variables|Character|GetMesh) 1 "/Game/Blueprints/Enemy/M_DissolveMaterial.M_DissolveMaterial" "None" :!class /Script/Engine.PrimitiveComponent))
  (bind _newtrack_0 (Timeline|Timeline_2 Play)
    (:Update
      (Rendering|Material|SetScalarParameterValue _returnvalue "Progress" _newtrack_0 :!class /Script/Engine.MaterialInstanceDynamic)
      (Utilities|FlowControl|Delay 1.5)
      (Rendering|Material|SetMaterial (Variables|Character|GetMesh) 1 "/Game/Project/DefaultStuff/Characters/Mannequins/Materials/Instances/Quinn/MI_Quinn_02.MI_Quinn_02")
      (Utilities|FlowControl|Delay 3.0))))

(event Custom|ded
  (Physics|SetSimulatePhysics (Variables|Character|GetMesh) true)
  (CallFunction|2)
  (Collision|SetCollisionEnabled (Variables|Collision|GetCapsuleComponent) "NoCollision")
  (bind _returnvalue (Rendering|Material|CreateDynamicMaterialInstance (Variables|Character|GetMesh) 0 "/Game/Blueprints/Enemy/MI_DissolveMaterial_Inst.MI_DissolveMaterial_Inst" "None" :!class /Script/Engine.PrimitiveComponent))
  (bind _newtrack_0 (Timeline|Timeline_0 Play)
    (:Update
      (Rendering|Material|SetScalarParameterValue _returnvalue "Progress" _newtrack_0 :!class /Script/Engine.MaterialInstanceDynamic)
      (Utilities|FlowControl|Delay 1.5)
      (Actor|DestroyActor))))

(event Collision|EventActorBeginOverlap
  (params (OtherActor :type Actor%20Object%20Reference)))

(event EventBeginPlay
  (CallFunction|SpawnEffect)
  (Utilities|FlowControl|Delay 0.2)
  (AI|AIMoveTo self "0, 0, 0" (Game|GetPlayerCharacter 0) 5.0 false :!label _label
    (:then
      (Utilities|FlowControl|Delay 0.2)
      (goto _label))))

(fn ConstructionScript)