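; Kamikaze enemy that explodes to damage the player, with spawn, charge and death effects driven by timelines on dynamic materials across two mesh slots.
; Tick writes timer-based aggro and attack-range flags to the AI blackboard, while a sphere overlap slows movement near the player.
; Boom charges, then explodes with camera shake and player damage without a distance check, unless lethal damage has already ragdolled and dissolved the enemy.
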(event OnComponentBeginOverlap(Sphere1)
  (params (OverlappedComponent :type Primitive%20Component%20Object%20Reference) (OtherActor :type Actor%20Object%20Reference) (OtherComp :type Primitive%20Component%20Object%20Reference) (OtherBodyIndex :type Integer) (bFromSweep :type Boolean) (SweepResult :type Hit%20Result%20Structure%20%28by%20ref%29)))

(event OnComponentBeginOverlap(Sphere)
  (params (OverlappedComponent :type Primitive%20Component%20Object%20Reference) (OtherActor :type Actor%20Object%20Reference) (OtherComp :type Primitive%20Component%20Object%20Reference) (OtherBodyIndex :type Integer) (bFromSweep :type Boolean) (SweepResult :type Hit%20Result%20Structure%20%28by%20ref%29))
  ;[1 1 1 1 33] MovementSpeed
  (Utilities|Casting|CastToBP_FirstPersonCharacter OtherActor)
  (Variables|/Script/Engine.CharacterMovementComponent|SetMaxWalkSpeed (Variables|Character|GetCharacterMovement) 7.5e+02))

(event OnComponentEndOverlap(Sphere)
  (params (OverlappedComponent :type Primitive%20Component%20Object%20Reference) (OtherActor :type Actor%20Object%20Reference) (OtherComp :type Primitive%20Component%20Object%20Reference) (OtherBodyIndex :type Integer))
  ;[1 1 1 1 33] MovementSpeed
  (Utilities|Casting|CastToBP_FirstPersonCharacter OtherActor)
  (Variables|/Script/Engine.CharacterMovementComponent|SetMaxWalkSpeed (Variables|Character|GetCharacterMovement) 1.5e+03))

(event OnComponentEndOverlap(Sphere1)
  (params (OverlappedComponent :type Primitive%20Component%20Object%20Reference) (OtherActor :type Actor%20Object%20Reference) (OtherComp :type Primitive%20Component%20Object%20Reference) (OtherBodyIndex :type Integer)))

(event Custom|Damage
  (Variables|Default|SetEnemyHealth (- (Variables|Default|GetEnemyHealth) 1))
  (if (not (> (Variables|Default|GetEnemyHealth) 1))
    (Physics|SetSimulatePhysics (Variables|Character|GetMesh) true)
    (CallFunction|2)
    (Collision|SetCollisionEnabled (Variables|Collision|GetCapsuleComponent) "NoCollision")
    (bind _returnvalue (Rendering|Material|CreateDynamicMaterialInstance (Variables|Character|GetMesh) 0 "/Game/Project/DefaultStuff/Characters/Mannequins/Materials/Instances/Quinn/MI_Kamikaze_03.MI_Kamikaze_03" "None" :!class /Script/Engine.PrimitiveComponent))
    (bind _newtrack_0 (Timeline|Timeline_0 Play)
      (:Update
        (Rendering|Material|SetScalarParameterValue _returnvalue "Progress" _newtrack_0 :!class /Script/Engine.MaterialInstanceDynamic)
        (Utilities|FlowControl|Delay 1.5)
        (Actor|DestroyActor)))))

(event Custom|2
  (bind _returnvalue (Rendering|Material|CreateDynamicMaterialInstance (Variables|Character|GetMesh) 1 "/Game/Project/DefaultStuff/Characters/Mannequins/Materials/Instances/Quinn/MI_Kamikaze_04.MI_Kamikaze_04" "None" :!class /Script/Engine.PrimitiveComponent))
  (bind _newtrack_0 (Timeline|Timeline Play)
    (:Update
      (Rendering|Material|SetScalarParameterValue _returnvalue "Progress" _newtrack_0 :!class /Script/Engine.MaterialInstanceDynamic))))

(event Custom|SpawnEffect
  (CallFunction|Second)
  (bind _returnvalue (Rendering|Material|CreateDynamicMaterialInstance (Variables|Character|GetMesh) 0 "/Game/Project/DefaultStuff/Characters/Mannequins/Materials/Instances/Quinn/MI_Kamikaze_03.MI_Kamikaze_03" "None" :!class /Script/Engine.PrimitiveComponent))
  (bind _newtrack_0 (Timeline|Timeline_1 Play)
    (:Update
      (Rendering|Material|SetScalarParameterValue _returnvalue "Progress" _newtrack_0 :!class /Script/Engine.MaterialInstanceDynamic)
      (Utilities|FlowControl|Delay 1.5)
      (Rendering|Material|SetMaterial (Variables|Character|GetMesh) 0 "/Game/Project/DefaultStuff/Characters/Mannequins/Materials/Instances/Quinn/MI_Quinn_01.MI_Quinn_01"))))

(event Custom|Second
  (bind _returnvalue (Rendering|Material|CreateDynamicMaterialInstance (Variables|Character|GetMesh) 1 "/Game/Project/DefaultStuff/Characters/Mannequins/Materials/Instances/Quinn/MI_Kamikaze_04.MI_Kamikaze_04" "None" :!class /Script/Engine.PrimitiveComponent))
  (bind _newtrack_0 (Timeline|Timeline_2 Play)
    (:Update
      (Rendering|Material|SetScalarParameterValue _returnvalue "Progress" _newtrack_0 :!class /Script/Engine.MaterialInstanceDynamic)
      (Utilities|FlowControl|Delay 1.5)
      (Rendering|Material|SetMaterial (Variables|Character|GetMesh) 1 "/Game/Project/DefaultStuff/Characters/Mannequins/Materials/Instances/Quinn/MI_Quinn_02.MI_Quinn_02"))))

(event Custom|Explode1
  (bind _returnvalue (Rendering|Material|CreateDynamicMaterialInstance (Variables|Character|GetMesh) 1 "/Game/Blueprints/Enemy/MI_DissolveMaterial_Inst.MI_DissolveMaterial_Inst" "None" :!class /Script/Engine.PrimitiveComponent))
  (bind _newtrack_0 (Timeline|Timeline_5 Play)
    (:Update
      (Rendering|Material|SetScalarParameterValue _returnvalue "Progress" _newtrack_0 :!class /Script/Engine.MaterialInstanceDynamic)
      (CallFunction|Boom))))

(event Custom|Charge2
  (bind _returnvalue (Rendering|Material|CreateDynamicMaterialInstance (Variables|Character|GetMesh) 1 "/Game/Project/DefaultStuff/Characters/Mannequins/Materials/Instances/Quinn/MI_Kamikaze_04.MI_Kamikaze_04" "None" :!class /Script/Engine.PrimitiveComponent))
  (bind _newtrack_0 (Timeline|Timeline_6 Play)
    (:Update
      (Rendering|Material|SetScalarParameterValue _returnvalue "ExplosionParam" _newtrack_0 :!class /Script/Engine.MaterialInstanceDynamic))))

(event Custom|ExplosionPlayerDamage
  (bind _asbp_first_person_character (Utilities|Casting|CastToBP_FirstPersonCharacter (Game|GetPlayerCharacter 0)))
  (Default|GetDamage _asbp_first_person_character))

(event Custom|Boom
  ;[1 1 1] Explode
  (Utilities|FlowControl|DoOnce false
    (:Completed
      (CallFunction|Charge2)
      (bind _returnvalue (Rendering|Material|CreateDynamicMaterialInstance (Variables|Character|GetMesh) 0 "/Game/Project/DefaultStuff/Characters/Mannequins/Materials/Instances/Quinn/MI_Kamikaze_03.MI_Kamikaze_03" "None" :!class /Script/Engine.PrimitiveComponent))
      (bind _newtrack_0 (Timeline|Timeline_3 Play)
        (:Update
          (Rendering|Material|SetScalarParameterValue _returnvalue "ExplosionParam" _newtrack_0 :!class /Script/Engine.MaterialInstanceDynamic))
        (:Finished
          (if (not (Physics|IsSimulatingPhysics (Variables|Character|GetMesh) "None"))
            (Effects|SpawnEmitteratLocation "/Game/Project/DefaultStuff/StarterContent/Particles/P_Explosion.P_Explosion" (Transformation|GetActorLocation) "0, 0, 0" "3.000000,3.000000,3.000000")
            (Audio|PlaySoundatLocation "/Game/ThirdParty/SciFiWeapDark/Sound/RocketLauncher/Wavs/RocketLauncher_Explosion01.RocketLauncher_Explosion01" (Transformation|GetActorLocation) "0, 0, 0" 1.0 1.0 0.0 0 0 0 0)
            (Camera|PlayWorldCameraShake "/Game/Blueprints/CameraShake/CSBP/CSBP_CameraShake_KamikazeExplosion.CSBP_CameraShake_KamikazeExplosion_C" "0, 0, 0" 4444.0 44444.0)
            (CallFunction|ExplosionPlayerDamage)
            (CallFunction|Explode1)
            (bind _returnvalue_2 (Rendering|Material|CreateDynamicMaterialInstance (Variables|Character|GetMesh) 0 "/Game/Blueprints/Enemy/MI_DissolveMaterial_Inst.MI_DissolveMaterial_Inst" "None" :!class /Script/Engine.PrimitiveComponent))
            (bind _newtrack_0_2 (Timeline|Timeline_4 Play)
              (:Update
                (Rendering|Material|SetScalarParameterValue _returnvalue_2 "Progress" _newtrack_0_2 :!class /Script/Engine.MaterialInstanceDynamic))
              (:Finished
                (Actor|DestroyActor)))))))))

(event EventTick
  (params (DeltaSeconds :type Float%20%28single-precision%29))
  (bind _returnvalue (Utilities|Name|MakeLiteralName "BT_IsAggro"))
  (bind _self self)
  (bind _returnvalue_2 (AI|GetAIController _self))
  (bind _returnvalue_3 (AI|GetBlackboard _returnvalue_2))
  (Utilities|FlowControl|Sequence
    (:then_0
      (bind _output_get (Variables|Default|SetDistanceToThePlayer (Math|Vector|VectorLength (- (Transformation|GetActorLocation (Components|GetOwner)) (Transformation|GetActorLocation (Game|GetPlayerCharacter 0)))))))
    (:then_1
      (if (<= (Variables|Default|GetAggroTimeActual) (Variables|Default|GetAggroTime))
        (bind _output_get_2 (Variables|Default|SetAggroTimeActual (+ (Variables|Default|GetAggroTimeActual) DeltaSeconds)))
        (Development|PrintText (Utilities|Text|ToText(Float) _output_get_2 "HalfToEven"))
        (AI|Components|Blackboard|SetValueasBool _returnvalue_3 _returnvalue true)
        (else
          (Variables|Default|SetAggroTimeActual 0.0)
          (AI|Components|Blackboard|SetValueasBool _returnvalue_3 _returnvalue false))))
    (:then_2
      (Utilities|FlowControl|Sequence
        (:then_0
          (AI|Components|Blackboard|SetValueasBool (AI|GetBlackboard (AI|GetAIController self)) (Utilities|Name|MakeLiteralName "BT_InRange") (<= (Transformation|GetDistanceTo (Game|GetPlayerCharacter 0)) (Variables|Default|GetAttack%20Range))))))
    (:then_3
      (if (<= _output_get 6e+02)
        _))))

(event EventBeginPlay
  (CallFunction|SpawnEffect))

(fn ConstructionScript)