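; Kamikaze enemy that materializes on spawn, chases the player with looped AI MoveTo and explodes up close.
; An outer-named Sphere overlap lowers its walk speed, while Sphere1 starts a one-time charge ending in explosion effects and player damage if still in range.
; Weapon damage events drain health, then ragdoll, dissolve and destroy it, cancelling the blast.
; Timelines drive dynamic material parameters on both mesh slots for spawn, charge and dissolve visuals.
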(event OnComponentBeginOverlap(Sphere1)
  (params (OverlappedComponent :type Primitive%20Component%20Object%20Reference) (OtherActor :type Actor%20Object%20Reference) (OtherComp :type Primitive%20Component%20Object%20Reference) (OtherBodyIndex :type Integer) (bFromSweep :type Boolean) (SweepResult :type Hit%20Result%20Structure%20%28by%20ref%29))
  ;[1 1 1] CIs Player in Range for explosion
  (Variables|Default|SetisInRange? true)
  (Utilities|Casting|CastToBP_FirstPersonCharacter OtherActor)
  (Utilities|FlowControl|DoOnce false
    (:Completed
      (CallFunction|Charge2)
      (bind _returnvalue (Rendering|Material|CreateDynamicMaterialInstance (Variables|Character|GetMesh) 0 "/Game/Project/DefaultStuff/Characters/Mannequins/Materials/Instances/Quinn/MI_Kamikaze_03.MI_Kamikaze_03" "None" :!class /Script/Engine.PrimitiveComponent))
      (bind _newtrack_0 (Timeline|Timeline_3 Play)
        (:Update
          (Rendering|Material|SetScalarParameterValue _returnvalue "ExplosionParam" _newtrack_0 :!class /Script/Engine.MaterialInstanceDynamic))
        (:Finished
          (if (not (Physics|IsSimulatingPhysics (Variables|Character|GetMesh) "None"))
            (Effects|SpawnEmitteratLocation "/Game/Project/DefaultStuff/StarterContent/Particles/P_Explosion.P_Explosion" (Transformation|GetActorLocation) "0, 0, 0" "3.000000,3.000000,3.000000")
            (Audio|PlaySoundatLocation "/Game/ThirdParty/SciFiWeapDark/Sound/RocketLauncher/Wavs/RocketLauncher_Explosion01.RocketLauncher_Explosion01" (Transformation|GetActorLocation) "0, 0, 0" 1.0 1.0 0.0 0 0 0 0)
            (Camera|PlayWorldCameraShake "/Game/Blueprints/CameraShake/CSBP/CSBP_CameraShake_KamikazeExplosion.CSBP_CameraShake_KamikazeExplosion_C" "0, 0, 0" 4444.0 44444.0)
            (CallFunction|ExplosionPlayerDamage)
            (CallFunction|Explode1)
            (bind _returnvalue_2 (Rendering|Material|CreateDynamicMaterialInstance (Variables|Character|GetMesh) 0 "/Game/Blueprints/Enemy/MI_DissolveMaterial_Inst.MI_DissolveMaterial_Inst" "None" :!class /Script/Engine.PrimitiveComponent))
            (bind _newtrack_0_2 (Timeline|Timeline_4 Play)
              (:Update
                (Rendering|Material|SetScalarParameterValue _returnvalue_2 "Progress" _newtrack_0_2 :!class /Script/Engine.MaterialInstanceDynamic))
              (:Finished
                (Actor|DestroyActor)
                (Default|CallDestroyed)))))))))

(event OnComponentBeginOverlap(Sphere)
  (params (OverlappedComponent :type Primitive%20Component%20Object%20Reference) (OtherActor :type Actor%20Object%20Reference) (OtherComp :type Primitive%20Component%20Object%20Reference) (OtherBodyIndex :type Integer) (bFromSweep :type Boolean) (SweepResult :type Hit%20Result%20Structure%20%28by%20ref%29))
  ;[1 1 1 1 33] MovementSpeed
  (Utilities|Casting|CastToBP_FirstPersonCharacter OtherActor)
  (Variables|/Script/Engine.CharacterMovementComponent|SetMaxWalkSpeed (Variables|Character|GetCharacterMovement) 7.5e+02))

(event OnComponentEndOverlap(Sphere)
  (params (OverlappedComponent :type Primitive%20Component%20Object%20Reference) (OtherActor :type Actor%20Object%20Reference) (OtherComp :type Primitive%20Component%20Object%20Reference) (OtherBodyIndex :type Integer))
  ;[1 1 1 1 33] MovementSpeed
  (Utilities|Casting|CastToBP_FirstPersonCharacter OtherActor)
  (Variables|/Script/Engine.CharacterMovementComponent|SetMaxWalkSpeed (Variables|Character|GetCharacterMovement) 1.5e+03))

(event OnComponentEndOverlap(Sphere1)
  (params (OverlappedComponent :type Primitive%20Component%20Object%20Reference) (OtherActor :type Actor%20Object%20Reference) (OtherComp :type Primitive%20Component%20Object%20Reference) (OtherBodyIndex :type Integer))
  ;[1 1 1] CIs Player in Range for explosion
  (Variables|Default|SetisInRange? false))

(event Custom|DamageShotgun
  (Variables|Default|SetEnemyHealth (- (Variables|Default|GetEnemyHealth) 8))
  (if (not (> (Variables|Default|GetEnemyHealth) 1))
    (Physics|SetSimulatePhysics (Variables|Character|GetMesh) true)
    (CallFunction|2)
    (Collision|SetCollisionEnabled (Variables|Collision|GetCapsuleComponent) "NoCollision")
    (bind _returnvalue (Rendering|Material|CreateDynamicMaterialInstance (Variables|Character|GetMesh) 0 "/Game/Project/DefaultStuff/Characters/Mannequins/Materials/Instances/Quinn/MI_Kamikaze_03.MI_Kamikaze_03" "None" :!class /Script/Engine.PrimitiveComponent))
    (bind _newtrack_0 (Timeline|Timeline_7 Play)
      (:Update
        (Rendering|Material|SetScalarParameterValue _returnvalue "Progress" _newtrack_0 :!class /Script/Engine.MaterialInstanceDynamic)
        (Utilities|FlowControl|Delay 1.5)
        (Actor|DestroyActor)
        (Default|CallDestroyed)))))

(event Custom|2
  ;[1 1 1] Dissolve Effect Explosion
  ;;[1 1 1] Second Material Effect
  (bind _returnvalue (Rendering|Material|CreateDynamicMaterialInstance (Variables|Character|GetMesh) 1 "/Game/Project/DefaultStuff/Characters/Mannequins/Materials/Instances/Quinn/MI_Kamikaze_04.MI_Kamikaze_04" "None" :!class /Script/Engine.PrimitiveComponent))
  (bind _newtrack_0 (Timeline|Timeline_0 Play)
    (:Update
      (Rendering|Material|SetScalarParameterValue _returnvalue "Progress" _newtrack_0 :!class /Script/Engine.MaterialInstanceDynamic))))

(event Custom|SpawnEffect
  (CallFunction|Second)
  (bind _returnvalue (Rendering|Material|CreateDynamicMaterialInstance (Variables|Character|GetMesh) 0 "/Game/Project/DefaultStuff/Characters/Mannequins/Materials/Instances/Quinn/MI_Kamikaze_03.MI_Kamikaze_03" "None" :!class /Script/Engine.PrimitiveComponent))
  (bind _newtrack_0 (Timeline|Timeline_1 Play)
    (:Update
      (Rendering|Material|SetScalarParameterValue _returnvalue "Progress" _newtrack_0 :!class /Script/Engine.MaterialInstanceDynamic)
      (Utilities|FlowControl|Delay 1.5)
      (Rendering|Material|SetMaterial (Variables|Character|GetMesh) 0 "/Game/Project/DefaultStuff/Characters/Mannequins/Materials/Instances/Quinn/MI_Quinn_01.MI_Quinn_01"))))

(event Custom|Second
  (bind _returnvalue (Rendering|Material|CreateDynamicMaterialInstance (Variables|Character|GetMesh) 1 "/Game/Project/DefaultStuff/Characters/Mannequins/Materials/Instances/Quinn/MI_Kamikaze_04.MI_Kamikaze_04" "None" :!class /Script/Engine.PrimitiveComponent))
  (bind _newtrack_0 (Timeline|Timeline_2 Play)
    (:Update
      (Rendering|Material|SetScalarParameterValue _returnvalue "Progress" _newtrack_0 :!class /Script/Engine.MaterialInstanceDynamic)
      (Utilities|FlowControl|Delay 1.5)
      (Rendering|Material|SetMaterial (Variables|Character|GetMesh) 1 "/Game/Project/DefaultStuff/Characters/Mannequins/Materials/Instances/Quinn/MI_Quinn_02.MI_Quinn_02"))))

(event Custom|Explode1
  (bind _returnvalue (Rendering|Material|CreateDynamicMaterialInstance (Variables|Character|GetMesh) 1 "/Game/Blueprints/Enemy/MI_DissolveMaterial_Inst.MI_DissolveMaterial_Inst" "None" :!class /Script/Engine.PrimitiveComponent))
  (bind _newtrack_0 (Timeline|Timeline_5 Play)
    (:Update
      (Rendering|Material|SetScalarParameterValue _returnvalue "Progress" _newtrack_0 :!class /Script/Engine.MaterialInstanceDynamic))))

(event Custom|Charge2
  (bind _returnvalue (Rendering|Material|CreateDynamicMaterialInstance (Variables|Character|GetMesh) 1 "/Game/Project/DefaultStuff/Characters/Mannequins/Materials/Instances/Quinn/MI_Kamikaze_04.MI_Kamikaze_04" "None" :!class /Script/Engine.PrimitiveComponent))
  (bind _newtrack_0 (Timeline|Timeline_6 Play)
    (:Update
      (Rendering|Material|SetScalarParameterValue _returnvalue "ExplosionParam" _newtrack_0 :!class /Script/Engine.MaterialInstanceDynamic))))

(event Custom|ExplosionPlayerDamage
  ;[1 1 1] Damage Player
  (if (Variables|Default|GetisInRange?)
    (bind _asbp_first_person_character (Utilities|Casting|CastToBP_FirstPersonCharacter (Game|GetPlayerCharacter 0)))
    (Default|GetDamage _asbp_first_person_character)))

(event Custom|Damage
  ;[1 1 1] Dissolve Effect Explosion
  ;;[1 1 1] Explosion Dissolve Effect
  (Variables|Default|SetEnemyHealth (- (Variables|Default|GetEnemyHealth) 20))
  (if (not (> (Variables|Default|GetEnemyHealth) 1))
    (Physics|SetSimulatePhysics (Variables|Character|GetMesh) true)
    (CallFunction|2)
    (Collision|SetCollisionEnabled (Variables|Collision|GetCapsuleComponent) "NoCollision")
    (bind _returnvalue (Rendering|Material|CreateDynamicMaterialInstance (Variables|Character|GetMesh) 0 "/Game/Project/DefaultStuff/Characters/Mannequins/Materials/Instances/Quinn/MI_Kamikaze_03.MI_Kamikaze_03" "None" :!class /Script/Engine.PrimitiveComponent))
    (bind _newtrack_0 (Timeline|Timeline Play)
      (:Update
        (Rendering|Material|SetScalarParameterValue _returnvalue "Progress" _newtrack_0 :!class /Script/Engine.MaterialInstanceDynamic)
        (Utilities|FlowControl|Delay 1.5)
        (Actor|DestroyActor)
        (Default|CallDestroyed)))))

(event Custom|DamagePlasmaRifle
  (Variables|Default|SetEnemyHealth (- (Variables|Default|GetEnemyHealth) 8))
  (if (not (> (Variables|Default|GetEnemyHealth) 1))
    (Physics|SetSimulatePhysics (Variables|Character|GetMesh) true)
    (CallFunction|2)
    (Collision|SetCollisionEnabled (Variables|Collision|GetCapsuleComponent) "NoCollision")
    (bind _returnvalue (Rendering|Material|CreateDynamicMaterialInstance (Variables|Character|GetMesh) 0 "/Game/Project/DefaultStuff/Characters/Mannequins/Materials/Instances/Quinn/MI_Kamikaze_03.MI_Kamikaze_03" "None" :!class /Script/Engine.PrimitiveComponent))
    (bind _newtrack_0 (Timeline|Timeline_8 Play)
      (:Update
        (Rendering|Material|SetScalarParameterValue _returnvalue "Progress" _newtrack_0 :!class /Script/Engine.MaterialInstanceDynamic)
        (Utilities|FlowControl|Delay 1.5)
        (Actor|DestroyActor)
        (Default|CallDestroyed)))))

(event EventBeginPlay
  (CallFunction|SpawnEffect)
  (Utilities|FlowControl|Delay 0.2)
  (AI|AIMoveTo self "0, 0, 0" (Game|GetPlayerCharacter 0) 5.0 false :!label _label
    (:then
      (Utilities|FlowControl|Delay 0.2)
      (goto _label))))

(fn ConstructionScript)