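; BP_VfxActor is a parent Blueprint actor that plays a configurable Niagara effect.
; Its construction script assigns the chosen Niagara asset to its component, resetting existing overrides, and feeds the Scale variable into the system's Scale parameter.
; On BeginPlay, a non-repeating effect destroys its actor after a fixed five-second delay, while a repeating one stays in the world.
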(event EventBeginPlay
  (if (not (Variables|Components|GetRepeating))
    (Utilities|FlowControl|Delay 5.0)
    (Actor|DestroyActor)))

(event Collision|EventActorBeginOverlap
  (params (OtherActor :type Actor%20Object%20Reference)))

(event EventTick
  (params (DeltaSeconds :type Float%20%28single-precision%29)))

(fn ConstructionScript
  (bind _niagaraasset (Variables|Components|GetNiagaraAsset))
  (if (Utilities|IsValid _niagaraasset)
    (Class|NiagaraComponent|SetAsset (Variables|Default|GetNiagaraSysstem) _niagaraasset true)
    (Niagara|SetNiagaraVariable(Float) (Variables|Default|GetNiagaraSysstem) "Scale" (Variables|Components|GetScale))))