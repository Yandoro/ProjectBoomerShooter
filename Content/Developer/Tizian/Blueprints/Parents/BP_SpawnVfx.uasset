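; Developer VFX preview actor that shows one effect at a time from ArrayOfVFXs, starting with the first on BeginPlay.
; Keys 1 and 2 step backward and forward through the array with wraparound, while Enter respawns the current effect.
; Each swap destroys all actors of the current class before spawning at this actor's X/Y, taking Z and rotation from that class's default HeightOffset and RotationOffset.
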(event EventBeginPlay
  (bind _returnvalue (Transformation|GetActorTransform))
  (bind _currentvfx (Variables|Components|GetCurrentVfx))
  (bind _returnvalue_2 (Math|Transform|TransformLocation _returnvalue "0, 0, 0"))
  (bind (_niagaraasset _repeating _heightoffset _scale _rotationoffset) (Utilities|GetClassDefaults _currentvfx))
  (bind (_x _y) (Math|Vector|BreakVector _returnvalue_2))
  (Input|EnableInput (Class|GameplayStatics|GetPlayerControllerfromID))
  (Game|SpawnActorfromClass _currentvfx (Math|Transform|MakeTransform (Math|Vector|MakeVector _x _y _heightoffset) _rotationoffset) "Undefined" "MultiplyWithRoot" 0 0))

(event Input|KeyboardEvents|1
  (params (Key :type Key%20Structure :default "None"))
  (bind _returnvalue (Transformation|GetActorTransform))
  (bind _returnvalue_2 (Math|Transform|TransformLocation _returnvalue "0, 0, 0"))
  (bind (_x _y) (Math|Vector|BreakVector _returnvalue_2))
  (:Pressed
    (bind _outactors (Actor|GetAllActorsOfClass (Variables|Components|GetCurrentVfx)))
    (Actor|DestroyActor _outactors)
    (if (<= (- (Variables|Components|Getid) 1) -1)
      (Variables|Components|Setid (- (Utilities|Array|Length (Variables|Components|GetArrayOfVFXs)) 1))
      (else
        (Variables|Components|Setid (- (Variables|Components|Getid) 1))))
    (bind _output_get (Variables|Components|SetCurrentVfx (Utilities|Array|Get(acopy) (Variables|Components|GetArrayOfVFXs) (Variables|Components|Getid))))
    (Game|SpawnActorfromClass _output_get (Math|Transform|MakeTransform (Math|Vector|MakeVector _x _y (.HeightOffset (Utilities|GetClassDefaults _output_get))) (.RotationOffset (Utilities|GetClassDefaults _output_get))) "Undefined" "MultiplyWithRoot" 0 0)))

(event Input|KeyboardEvents|2
  (params (Key :type Key%20Structure :default "None"))
  (bind _returnvalue (Transformation|GetActorTransform))
  (bind _returnvalue_2 (Math|Transform|TransformLocation _returnvalue "0, 0, 0"))
  (bind (_x _y) (Math|Vector|BreakVector _returnvalue_2))
  (:Pressed
    (bind _outactors (Actor|GetAllActorsOfClass (Variables|Components|GetCurrentVfx)))
    (Actor|DestroyActor _outactors)
    (if (>= (+ (Variables|Components|Getid) 1) (Utilities|Array|Length (Variables|Components|GetArrayOfVFXs)))
      (Variables|Components|Setid 0)
      (else
        (Variables|Components|Setid (Math|Conversions|ToInteger(Byte) (+ (Variables|Components|Getid) 1)))))
    (bind _output_get (Variables|Components|SetCurrentVfx (Utilities|Array|Get(acopy) (Variables|Components|GetArrayOfVFXs) (Variables|Components|Getid))))
    (Game|SpawnActorfromClass _output_get (Math|Transform|MakeTransform (Math|Vector|MakeVector _x _y (.HeightOffset (Utilities|GetClassDefaults _output_get))) (.RotationOffset (Utilities|GetClassDefaults _output_get))) "Undefined" "MultiplyWithRoot" 0 0)))

(event Input|KeyboardEvents|Enter
  (params (Key :type Key%20Structure :default "None"))
  (bind _returnvalue (Transformation|GetActorTransform))
  (bind _currentvfx (Variables|Components|GetCurrentVfx))
  (bind _returnvalue_2 (Math|Transform|TransformLocation _returnvalue "0, 0, 0"))
  (bind (_niagaraasset _repeating _heightoffset _scale _rotationoffset) (Utilities|GetClassDefaults _currentvfx))
  (bind (_x _y) (Math|Vector|BreakVector _returnvalue_2))
  (:Pressed
    (bind _outactors (Actor|GetAllActorsOfClass (Variables|Components|GetCurrentVfx)))
    (Actor|DestroyActor _outactors)
    (Game|SpawnActorfromClass _currentvfx (Math|Transform|MakeTransform (Math|Vector|MakeVector _x _y _heightoffset) _rotationoffset) "Undefined" "MultiplyWithRoot" 0 0)))

(fn ConstructionScript
  (bind _output_get (Variables|Components|Setid 0))
  (Variables|Components|SetCurrentVfx (Utilities|Array|Get(acopy) (Variables|Components|GetArrayOfVFXs) _output_get)))