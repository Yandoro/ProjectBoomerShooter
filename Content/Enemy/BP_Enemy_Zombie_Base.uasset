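; Base zombie enemy that chases the player and dissolves in on spawn and out on death.
; BeginPlay runs timeline-driven dissolves on both mesh material slots, restores the Quinn materials, and reissues AIMoveTo on a short delay loop.
; A sphere overlap halves walk speed while the player is inside.
; Damage decrements health and, at one or below, ragdolls the mesh, disables capsule collision, dissolves it and destroys the actor.
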(event OnComponentBeginOverlap(Sphere)
  (params (OverlappedComponent :type Primitive%20Component%20Object%20Reference) (OtherActor :type Actor%20Object%20Reference) (OtherComp :type Primitive%20Component%20Object%20Reference) (OtherBodyIndex :type Integer) (bFromSweep :type Boolean) (SweepResult :type Hit%20Result%20Structure%20%28by%20ref%29))
  (Utilities|Casting|CastToBP_FirstPersonCharacter OtherActor)
  (Variables|/Script/Engine.CharacterMovementComponent|SetMaxWalkSpeed (Variables|Character|GetCharacterMovement) 7.5e+02))

(event OnComponentEndOverlap(Sphere)
  (params (OverlappedComponent :type Primitive%20Component%20Object%20Reference) (OtherActor :type Actor%20Object%20Reference) (OtherComp :type Primitive%20Component%20Object%20Reference) (OtherBodyIndex :type Integer))
  (Utilities|Casting|CastToBP_FirstPersonCharacter OtherActor)
  (Variables|/Script/Engine.CharacterMovementComponent|SetMaxWalkSpeed (Variables|Character|GetCharacterMovement) 1.5e+03))

(event Custom|Damage
  (Variables|Default|SetEnemyHealth (- (Variables|Default|GetEnemyHealth) 1))
  (if (not (> (Variables|Default|GetEnemyHealth) 1))
    (Physics|SetSimulatePhysics (Variables|Character|GetMesh) true)
    (CallFunction|2)
    (Collision|SetCollisionEnabled (Variables|Collision|GetCapsuleComponent) "NoCollision")
    (bind _returnvalue (Rendering|Material|CreateDynamicMaterialInstance (Variables|Character|GetMesh) 0 "/Game/Enemy/MI_DissolveMaterial_Inst.MI_DissolveMaterial_Inst" "None" :!class /Script/Engine.PrimitiveComponent))
    (bind _newtrack_0 (Timeline|Timeline_0 Play)
      (:Update
        (Rendering|Material|SetScalarParameterValue _returnvalue "Progress" _newtrack_0 :!class /Script/Engine.MaterialInstanceDynamic)
        (Utilities|FlowControl|Delay 1.5)
        (Actor|DestroyActor)))))

(event Custom|2
  (bind _returnvalue (Rendering|Material|CreateDynamicMaterialInstance (Variables|Character|GetMesh) 1 "/Game/Enemy/MI_DissolveMaterial_Inst.MI_DissolveMaterial_Inst" "None" :!class /Script/Engine.PrimitiveComponent))
  (bind _newtrack_0 (Timeline|Timeline Play)
    (:Update
      (Rendering|Material|SetScalarParameterValue _returnvalue "Progress" _newtrack_0 :!class /Script/Engine.MaterialInstanceDynamic))))

(event Custom|SpawnEffect
  (CallFunction|Second)
  (bind _returnvalue (Rendering|Material|CreateDynamicMaterialInstance (Variables|Character|GetMesh) 0 "/Game/Enemy/M_DissolveMaterial.M_DissolveMaterial" "None" :!class /Script/Engine.PrimitiveComponent))
  (bind _newtrack_0 (Timeline|Timeline_1 Play)
    (:Update
      (Rendering|Material|SetScalarParameterValue _returnvalue "Progress" _newtrack_0 :!class /Script/Engine.MaterialInstanceDynamic)
      (Utilities|FlowControl|Delay 1.5)
      (Rendering|Material|SetMaterial (Variables|Character|GetMesh) 0 "/Game/Characters/Mannequins/Materials/Instances/Quinn/MI_Quinn_01.MI_Quinn_01"))))

(event Custom|Second
  (bind _returnvalue (Rendering|Material|CreateDynamicMaterialInstance (Variables|Character|GetMesh) 1 "/Game/Enemy/M_DissolveMaterial.M_DissolveMaterial" "None" :!class /Script/Engine.PrimitiveComponent))
  (bind _newtrack_0 (Timeline|Timeline_2 Play)
    (:Update
      (Rendering|Material|SetScalarParameterValue _returnvalue "Progress" _newtrack_0 :!class /Script/Engine.MaterialInstanceDynamic)
      (Utilities|FlowControl|Delay 1.5)
      (Rendering|Material|SetMaterial (Variables|Character|GetMesh) 1 "/Game/Characters/Mannequins/Materials/Instances/Quinn/MI_Quinn_02.MI_Quinn_02"))))

(event Collision|EventActorBeginOverlap
  (params (OtherActor :type Actor%20Object%20Reference)))

(event EventBeginPlay
  (CallFunction|SpawnEffect)
  (Utilities|FlowControl|Delay 0.2)
  (AI|AIMoveTo self "0, 0, 0" (Game|GetPlayerCharacter 0) 5.0 false :!label _label
    (:then
      (Utilities|FlowControl|Delay 0.2)
      (goto _label))))

(fn ConstructionScript)